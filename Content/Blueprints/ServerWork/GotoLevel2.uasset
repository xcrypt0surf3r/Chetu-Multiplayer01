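; GotoLevel2 is a trigger-box actor that sends the first local player into another online session when its Box is overlapped, with no filter on the overlapping actor.
; The overlap prints the player's index, then runs a small non-LAN session search.
; On success it prints each result and joins the one at hardcoded index 1, with no count check or failure handling.
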(event OnComponentBeginOverlap(Box)
  (params (OverlappedComponent :type Primitive%20Component%20Object%20Reference) (OtherActor :type Actor%20Object%20Reference) (OtherComp :type Primitive%20Component%20Object%20Reference) (OtherBodyIndex :type Integer) (bFromSweep :type Boolean) (SweepResult :type Hit%20Result%20Structure%20%28by%20ref%29))
  (bind _returnvalue (Game|GetPlayerController 0))
  (bind _playerindex (Class|TurnBasedBlueprintLibrary|GetMyPlayerIndex _returnvalue))
  (Development|PrintString (Utilities|String|ToString(Integer) _playerindex))
  (bind _results (|FindSessions _returnvalue 5 false)
    (:OnSuccess
      (for (_ _array_index) _results
        (Development|PrintString (Utilities|String|ToString(Integer) _array_index)))
      (Development|PrintString "Thats All ")
      (|JoinSession (Game|GetPlayerController 0) (Utilities|Array|Get(acopy) _results 1)))))

(event EventBeginPlay)

(event Collision|EventActorBeginOverlap
  (params (OtherActor :type Actor%20Object%20Reference)))

(event EventTick
  (params (DeltaSeconds :type Float%20%28single-precision%29)))

(fn ConstructionScript)